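; BasicEnemyBP is a basic enemy with a configurable mesh that has hit points and is destroyed when they run out.
; HitPoints drop through AnyDamage or a custom Damage event, while player projectile hits briefly swap the body material as a flash.
; Any actor overlap subtracts a fixed amount from the player character's health, without checking what overlapped.
; The construction script applies the chosen mesh with a dynamic material instance, or prints a setup warning.
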(event Custom|HitFlash
  (Rendering|Material|SetMaterial (Variables|Default|GetBody) 0 "/Game/Adam/Misc/Materials/HitFlash.HitFlash")
  (Utilities|FlowControl|Delay 0.08)
  (Rendering|Material|SetMaterial (Variables|Default|GetBody) 0 (Variables|Default|GetMeshMat)))

(event Custom|Damage
  (bind _output_get (Variables|Default|SetHitPoints (- (Variables|Default|GetHitPoints) (Variables|Default|GetDamagePoints))))
  (Development|PrintString (Utilities|String|ToString(Float) _output_get))
  (if (<= (Variables|Default|GetHitPoints) 0.0)
    (Actor|DestroyActor)))

(event EventHit
  (params (MyComp :type Primitive%20Component%20Object%20Reference) (Other :type Actor%20Object%20Reference) (OtherComp :type Primitive%20Component%20Object%20Reference) (bSelfMoved :type Boolean) (HitLocation :type Vector :default "0, 0, 0") (HitNormal :type Vector :default "0, 0, 0") (NormalImpulse :type Vector :default "0, 0, 0") (Hit :type Hit%20Result%20Structure%20%28by%20ref%29))
  ;[1 1 1] Hit Flash
  (if (Actor|ActorHasTag Other "PlayerProjectile")
    (Utilities|FlowControl|Sequence
      (:then_0
        (Rendering|Material|SetMaterial (Variables|Default|GetBody) 0 "/Game/Adam/Misc/Materials/HitFlash.HitFlash")
        (Utilities|FlowControl|Delay 0.08)
        (Rendering|Material|SetMaterial (Variables|Default|GetBody) 0 (Variables|Default|GetMeshMat))))))

(event EventActorBeginOverlap
  (params (OtherActor :type Actor%20Object%20Reference))
  ;[1 1 1] Damage Character
  (bind _asthird_person_character (Utilities|Casting|CastToThirdPersonCharacter (Game|GetPlayerCharacter 0)))
  (Variables|/Game/ThirdPersonBP/Blueprints/ThirdPersonCharacter.ThirdPersonCharacter_C|SetCurrentHealth _asthird_person_character (- (Variables|/Game/ThirdPersonBP/Blueprints/ThirdPersonCharacter.ThirdPersonCharacter_C|GetCurrentHealth _asthird_person_character) 4e+01)))

(event EventAnyDamage
  (params (Damage :type Float%20%28single-precision%29) (DamageType :type Damage%20Type%20Object%20Reference) (InstigatedBy :type Controller%20Object%20Reference) (DamageCauser :type Actor%20Object%20Reference))
  ;[1 1 1] Damage
  (Variables|Default|SetHitPoints (- (Variables|Default|GetHitPoints) Damage))
  (if (<= (Variables|Default|GetHitPoints) 0.0)
    (Actor|DestroyActor)))

(fn ConstructionScript
  (bind _variablemesh (Variables|Default|GetVariableMesh))
  (if (== _variablemesh 0)
    (Development|PrintString "Please set VariableMesh before use")
    (else
      (Components|StaticMesh|SetStaticMesh (Variables|Default|GetBody) _variablemesh)
      (bind _returnvalue (Rendering|Material|CreateDynamicMaterialInstance (Variables|Default|GetMeshMat) :!class /Script/Engine.KismetMaterialLibrary))
      (Rendering|Material|SetMaterial (Variables|Default|GetBody) 0 _returnvalue))))